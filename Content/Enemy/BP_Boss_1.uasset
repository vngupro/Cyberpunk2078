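; BP_Boss_1 is an enemy boss character that tracks Health and takes damage.
; AnyDamage subtracts the incoming damage from Health, cut to a quarter while the SoonHit flag is set for badly timed hits.
; A death check with montage and movement stop, plus a delayed destroy, exists but is disconnected, so it never runs.
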(event `self.ReceiveAnyDamage`
  (params (Damage :type "Float (single-precision)") (DamageType :type "DamageType Object Reference") (InstigatedBy :type "Controller Object Reference") (DamageCauser :type "Actor Object Reference"))
  ;[1 1 1] Take Damage
  (`|ExecutionSequence`
    (:`then_0`
      (if (`self.SoonHit`)
        (set `self.Health` (- (`self.Health`) (/ Damage 4.0)))
        (else
          (set `self.Health` (- (`self.Health`) Damage)))))))

(fn `UserConstructionScript`
  (`parent.UserConstructionScript`))