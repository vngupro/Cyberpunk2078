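; Enemy with rhythm-timed hit windows, signalled by glow material changes on its head.
; Audiotest's envelope peaks, throttled by a cooldown, drive the windows; a second track starts after an offset, so Audiotest runs ahead.
; Damage is quartered during the early SoonHit phase; CanBeHit is set but never read here.
; Helpers cover projectile impact, health decrement and Blackboard-updating death, but the death check is unwired and Tick is empty.
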(event `self.ReceiveAnyDamage`
  (params (Damage :type "Float (single-precision)") (DamageType :type "DamageType Object Reference") (InstigatedBy :type "Controller Object Reference") (DamageCauser :type "Actor Object Reference"))
  ;[1 1 1] Damage
  (if (`self.SoonHit`)
    (set `self.Health` (- (`self.Health`) (/ Damage 4.0)))
    (else
      (set `self.Health` (- (`self.Health`) Damage)))))

(event `self.ReceiveBeginPlay`
  ;[1 1 1] setup
  (set `self.delay` (`self.InitialDelay`))
  (`AudioComponent.Play` (`self.Audiotest`) 0.0)
  (`KismetSystemLibrary.Delay` (`self.DelayBetweenPist`))
  (`AudioComponent.Play` (`self.Audio`) 0.0))

(event `self.Audio.OnAudioSingleEnvelopeValue`
  (params (PlayingSoundWave :type "SoundWave Object Reference") (EnvelopeValue :type "Float (single-precision)")))

(event `self.ReceiveTick`
  (params (DeltaSeconds :type "Float (single-precision)")))

(event `self.Audiotest.OnAudioSingleEnvelopeValue`
  (params (PlayingSoundWave :type "SoundWave Object Reference") (EnvelopeValue :type "Float (single-precision)"))
  (bind _timing (`self.Timing`))
  (bind _delay (`self.delay`))
  (bind _head (`self.Head`))
  (if (and (> EnvelopeValue 0.06) (<= _delay 0.0))
    (set `self.delay` (`self.InitialDelay`))
    (`KismetSystemLibrary.Delay` _timing)
    (set `self.CanBeHit` true)
    (set `self.SoonHit` true)
    (`PrimitiveComponent.SetMaterial` _head 1 "/Game/FirstPersonBP/Blueprints/Glow.Glow")
    (`KismetSystemLibrary.Delay` _timing)
    (set `self.SoonHit` false)
    (`PrimitiveComponent.SetMaterial` _head 1 "/Game/FirstPersonBP/Blueprints/GreenGlow.GreenGlow")
    (`KismetSystemLibrary.Delay` 0.5)
    (`PrimitiveComponent.SetMaterial` _head 1 "/Game/FirstPersonBP/Blueprints/RedGlow.RedGlow")
    (set `self.CanBeHit` false)
    (else
      (set `self.delay` (- _delay (`GameplayStatics.GetWorldDeltaSeconds`))))))

(fn `Die`
  (`MovementComponent.StopMovementImmediately` (`self.CharacterMovement`))
  (`SkeletalMeshComponent.PlayAnimation` (`self.Mesh`) "/Game/AnimBoss/Boss_Death.Boss_Death" false)
  (bind _asenemy_controller (cast `/Game/Enemy/Old/Enemy_Controller` (`self.GetController`)))
  (bind _output_get (set `self.State` "NewEnumerator7"))
  (`BlackboardComponent.SetValueAsEnum` (`AIBlueprintHelperLibrary.GetBlackboard` _asenemy_controller) "Status" _output_get))

(fn `TakeHit`
  (params (`Hit Actor` :type "Actor Object Reference"))
  (bind _hitparticle (`self.HitParticle`))
  (bind _asfirst_person_projectile (cast `/Game/FirstPersonBP/Blueprints/FirstPersonProjectile` `Hit Actor`))
  (`SceneComponent.K2_SetWorldLocation` _hitparticle (`SceneComponent.K2_GetComponentLocation` (`/Game/FirstPersonBP/Blueprints/FirstPersonProjectile.Sphere` _asfirst_person_projectile)) false false)
  (`ActorComponent.Activate` _hitparticle true)
  (`self.K2_DestroyActor` _asfirst_person_projectile) ; Destroy Projectile
)

(fn `UpdateHealth`
  (params (Damage :type "Float (double-precision)"))
  (set `self.Health` (- (`self.Health`) 1.0)) ; Update Health
)

(fn `UserConstructionScript`
  (set `self.Health` (`self.Max_Health`)))