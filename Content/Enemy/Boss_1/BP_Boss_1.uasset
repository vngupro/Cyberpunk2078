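; Boss 1 enemy Blueprint that extends its parent's attack event with an energy burst AoE attack.
; AttackEvent spawns BP_EnergyBurst and plays a montage whose notifies start charge sound and particles, then clear them and cast the ability.
; The random attack switch has only the AoE case wired, while a Fireball attack sits disconnected and never runs.
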(event `self.AttackEvent`
  (bind (_returnvalue_x _returnvalue_y) (`KismetMathLibrary.BreakVector` (`self.K2_GetActorLocation`)))
  (bind _action_chargeaoe_animmontage (break `/Game/Enemy/SAction` (`self.Action_ChargeAoE`)))
  (bind (_action_chargeaoe_animmontage_2 _action_chargeaoe_particle _action_chargeaoe_sound) (break `/Game/Enemy/SAction` (`self.Action_ChargeAoE`)))
  (bind (_action_aoe_animmontage _action_aoe_particle _action_aoe_sound) (break `/Game/Enemy/SAoE` (`self.Action_AoE`)))
  (bind (_action_chargeaoe_animmontage_3 _action_chargeaoe_particle_2) (break `/Game/Enemy/SAction` (`self.Action_ChargeAoE`)))
  ;[1 1 1] Attack
  (`parent.AttackEvent`)
  (`|ExecutionSequence`
    (:`then_0`
      (switch `int` (`KismetMathLibrary.RandomInteger` 0)
        (:`0`
          ;;[1 1 1] AoE
          (bind _returnvalue (`|SpawnActorFromClass` "/Game/Enemy/AbilitySystem/Aoe/BP_EnergyBurst.BP_EnergyBurst_C" (`self.GetTransform`) "Undefined" "OverrideRootScale" null self null))
          (`KismetSystemLibrary.PrintString` "energy burst")
          (bind _notifyname (`|PlayMontage` (`self.Mesh`) _action_chargeaoe_animmontage 1.0 0.0 "None")
            (:`OnNotifyBegin`
              (if (== _notifyname "ChargeAoE")
                (bind _returnvalue_2 (`GameplayStatics.SpawnSound2D` _action_chargeaoe_sound 1.0 1.0 0.0 null))
                (bind _returnvalue_3 (`GameplayStatics.SpawnEmitterAtLocation` _action_chargeaoe_particle_2 (`KismetMathLibrary.MakeVector` _returnvalue_x _returnvalue_y)))
                (elif (== _notifyname "CastSpell")
                  (`GameplayStatics.PlaySound2D` _action_aoe_sound 1.0 1.0 0.0 null null)
                  (`ActorComponent.K2_DestroyComponent` _returnvalue_2)
                  (`ActorComponent.K2_DestroyComponent` _returnvalue_3)
                  (`/Game/Enemy/AbilitySystem/BP_Ability.CastAbility` _returnvalue))))))))))

(event `self.ReceiveBeginPlay`
  ;[1 1 1] Attack
  (`parent.ReceiveBeginPlay`))

(fn `UserConstructionScript`
  (`parent.UserConstructionScript`))