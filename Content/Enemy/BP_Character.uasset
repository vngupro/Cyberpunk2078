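; Enemy character, apparently a base given its empty AttackEvent, that handles health, hit reactions and death.
; AnyDamage always subtracts a quarter of the damage (HitNotInTiming branch fixed to true), then spawns temporary hit particles.
; ActionHit and ActionDeath data drive the hit montage or the death animation, effect and sound, with IAmDead called after a delay.
; Tick derives HasEndAttack from montage playback; destruction clears leftover particles.
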(event `self.ReceiveAnyDamage`
  (params (Damage :type "Float (single-precision)") (DamageType :type "DamageType Object Reference") (InstigatedBy :type "Controller Object Reference") (DamageCauser :type "Actor Object Reference"))
  (bind (_actionhit_animmontage _actionhit_particle _actionhit_sound _actionhit_particledestroydelay) (break `/Game/Enemy/SAction` (`self.ActionHit`)))
  (bind (_actiondeath_animseq _actiondeath_particle _actiondeath_sound _actiondeath_particledestroydelay) (break `/Game/Enemy/SDeath` (`self.ActionDeath`)))
  (bind (_returnvalue_x _returnvalue_y _returnvalue_z) (`KismetMathLibrary.BreakVector` (`SceneComponent.K2_GetComponentLocation` (`self.Mesh`))))
  ;[1 1 1] Take Damage
  (`|ExecutionSequence`
    (:`then_0`
      (if true
        (set `self.Health` (- (`self.Health`) (/ Damage 4.0)))
        (else
          (set `self.Health` (- (`self.Health`) Damage)))))
    (:`then_1`
      (bind _particleref (`/Game/Enemy/BPL_Boss.TakeHit` _actionhit_particle (`self.HitLocation`)))
      (`KismetArrayLibrary.Array_Add` (`self.ParticleArr`) _particleref)
      (`KismetSystemLibrary.Delay` _actionhit_particledestroydelay)
      (for _array_element (`self.ParticleArr`)
        (`/Engine/EditorBlueprintResources/StandardMacros.IsValid` _array_element
          (:`Is Valid`
            (`ActorComponent.K2_DestroyComponent` _particleref)
            (`ActorComponent.K2_DestroyComponent` _array_element))))
      (`KismetArrayLibrary.Array_Clear` (`self.ParticleArr`)))
    (:`then_2`
      (if (> (`self.Health`) 0.0)
        (if (not (`AnimInstance.IsAnyMontagePlaying` (`SkeletalMeshComponent.GetAnimInstance` (`self.Mesh`))))
          (`|PlayMontage` (`self.Mesh`) _actionhit_animmontage))
        (else
          (`MovementComponent.StopMovementImmediately` (`self.CharacterMovement`))
          (`SkeletalMeshComponent.PlayAnimation` (`self.Mesh`) _actiondeath_animseq false)
          (bind _returnvalue (`GameplayStatics.SpawnEmitterAtLocation` _actiondeath_particle (`KismetMathLibrary.MakeVector` _returnvalue_x _returnvalue_y _returnvalue_z)))
          (`GameplayStatics.PlaySound2D` _actiondeath_sound 1.0 1.0 0.0 null null)
          (`KismetSystemLibrary.Delay` _actiondeath_particledestroydelay)
          (`ActorComponent.K2_DestroyComponent` _returnvalue)
          (`self.IAmDead`))))))

(event `self.ReceiveBeginPlay`
  ;[1 1 1] Init
  (`|ExecutionSequence`
    (:`then_0`
      ;;[1 1 1] Set Health
      (set `self.Target` (`GameplayStatics.GetPlayerCharacter` 0))
      (set `self.Health` (`self.MaxHealth`))
      (add `self.OnDestroyed` (delegate `CustomEvent_0`)))))

(event `CustomEvent_0` :!signature `self.OnDestroyed`
  (params (DestroyedActor :type "Actor Object Reference"))
  (for _array_element (`self.ParticleArr`)
    (`/Engine/EditorBlueprintResources/StandardMacros.IsValid` _array_element
      (:`Is Valid`
        (`ActorComponent.K2_DestroyComponent` _array_element)
        (`KismetArrayLibrary.Array_Clear` (`self.ParticleArr`) :!label _label))))
  (goto _label))

(event `AttackEvent`
  ;[1 1 1] Attack
)

(event `self.ReceiveTick`
  (params (DeltaSeconds :type "Float (single-precision)"))
  ;[1 1 1] Attack
  (if (`AnimInstance.IsAnyMontagePlaying` (`SkeletalMeshComponent.GetAnimInstance` (`self.Mesh`)))
    (set `self.hasEndAttack` false)
    (else
      (set `self.hasEndAttack` true))))

(fn `UserConstructionScript`
  (set `self.Health` (`self.MaxHealth`)))