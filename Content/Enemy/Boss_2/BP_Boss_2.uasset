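; Second boss enemy that rotates through four spell attacks and can be hit in windows timed to music.
; AttackEvent uses flags to cycle fireball, spread, homing and AoE burst, spawning spell actors and casting them from montage notifies.
; An audio envelope on the Beat track opens hit windows, signaled by material swaps and a player UI marker.
; Tick handles the beat cooldown and retunes window timing later in the fight.
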(event `self.AttackEvent`
  (bind _returnvalue (`self.GetTransform`))
  (bind _returnvalue_2 (`self.GetTransform`))
  (bind (_returnvalue_x _returnvalue_y _returnvalue_z) (`KismetMathLibrary.BreakVector` (`self.K2_GetActorLocation`)))
  (bind _returnvalue_3 (`self.GetTransform`))
  (bind (_returnvalue_roll _returnvalue_pitch _returnvalue_yaw) (`KismetMathLibrary.BreakRotator` (`self.K2_GetActorRotation`)))
  (bind (_sspread_animmontage _sspread_particle _sspread_sound) (break `/Game/Enemy/SAction` (`self.SSpread`)))
  (bind (_shoming_animmontage _shoming_particle _shoming_sound) (break `/Game/Enemy/SAction` (`self.SHoming`)))
  (bind _saoecharge_animmontage (break `/Game/Enemy/SAction` (`self.SAoECharge`)))
  (bind (_saoecharge_animmontage_2 _saoecharge_particle _saoecharge_sound) (break `/Game/Enemy/SAction` (`self.SAoECharge`)))
  (bind _shoming_animmontage_2 (break `/Game/Enemy/SAction` (`self.SHoming`)))
  (bind _sspread_animmontage_2 (break `/Game/Enemy/SAction` (`self.SSpread`)))
  (bind (_sfireball_animmontage _sfireball_particle _sfireball_sound) (break `/Game/Enemy/SAction` (`self.SFireball`)))
  (bind _spreadangle (`self.SpreadAngle`))
  (bind _homingarr (`self.HomingArr`))
  (bind _spreadangle_2 (`self.SpreadAngle`))
  (bind _returnvalue_4 (`KismetMathLibrary.RandomFloatInRange` (`self.HMinScale`) (`self.HMaxScale`)))
  (bind _returnvalue_5 (`SceneComponent.GetRelativeTransform` (`self.CapsuleComponent`)))
  ;[1 1 1] Attack
  (`parent.AttackEvent`)
  (if (`self.didFireball`)
    (if (`self.didSpread`)
      (if (`self.didHoming`)
        (`|ExecutionSequence`
          (:`then_0`
            ;;[1 1 1] AoE
            (bind _returnvalue_6 (`|SpawnActorFromClass` "/Game/Enemy/AbilitySystem/Aoe/BP_EnergyBurst2.BP_EnergyBurst2_C" (`KismetMathLibrary.MakeTransform` (`KismetMathLibrary.MakeVector` (.x (.location _returnvalue_2)) (.y (.location _returnvalue_2)) (+ (.z (.location _returnvalue_2)) (`self.AoEZOffset`))) (.rotation _returnvalue_2) (.scale _returnvalue_2)) "Undefined" "OverrideRootScale" null self null))
            (set `self.AoERef` _returnvalue_6)
            (bind _notifyname (`|PlayMontage` (`self.Mesh`) _saoecharge_animmontage 1.0 0.0 "None")
              (:`OnInterrupted`
                (bind _aoeref (`self.AoERef`)
                  (:`then`
                    (`self.K2_DestroyActor` _aoeref))
                  (:`else`)))
              (:`OnNotifyBegin`
                (if (== _notifyname "ChargeAoE")
                  (bind _returnvalue_7 (`GameplayStatics.SpawnSound2D` _saoecharge_sound 1.0 1.0 0.0 null))
                  (set `self.AoESoundRef` _returnvalue_7)
                  (bind _returnvalue_8 (`GameplayStatics.SpawnEmitterAtLocation` _saoecharge_particle (`KismetMathLibrary.MakeVector` _returnvalue_x _returnvalue_y (+ _returnvalue_z (`self.AoEZOffset`)))))
                  (set `self.AoEParticleRef` _returnvalue_8)
                  (elif (== _notifyname "CastSpell")
                    (`GameplayStatics.PlaySound2D` "/Game/StarterContent/Audio/Explosion_Cue.Explosion_Cue" 1.0 1.0 0.0 null null)
                    (bind _aoesoundref (`self.AoESoundRef`)
                      (:`then`
                        (`ActorComponent.K2_DestroyComponent` _aoesoundref))
                      (:`else`
                        _))
                    (bind _aoeparticleref (`self.AoEParticleRef`)
                      (:`then`
                        (`ActorComponent.K2_DestroyComponent` _aoeparticleref)
                        (bind _aoeref_2 (`self.AoERef`)
                          (:`then`
                            _)
                          (:`else`)))
                      (:`else`
                        _))
                    (`/Game/Enemy/AbilitySystem/BP_Ability.CastAbility` _aoeref_2))))))
          (:`then_1`
            (set `self.didFireball` false)
            (set `self.didSpread` false)
            (set `self.didHoming` false)))
        (else
          (`|ExecutionSequence`
            (:`then_0`
              ;;[1 1 1] Homing
              (`KismetArrayLibrary.Array_Clear` (`self.HomingArr`))
              (for _index (range (+ (`self.NbHoming`) 1))
                (if (== (mod _index 2) 0)
                  (`GameplayStatics.PlaySound2D` _shoming_sound 1.0 1.0 0.0 null null))
                (bind _returnvalue_9 (`|SpawnActorFromClass` "/Game/Enemy/AbilitySystem/Projectiles/BP_Homing.BP_Homing_C" (`KismetMathLibrary.MakeTransform` (`KismetMathLibrary.MakeVector` (+ (.x (.location _returnvalue_5)) (`KismetMathLibrary.RandomFloatInRange` (`self.HSpawnXMinOffset`) (`self.HSpawnXMaxOffset`))) (+ (.y (.location _returnvalue_5)) (`KismetMathLibrary.RandomFloatInRange` (`self.HSpawnYMinOffset`) (`self.HSpawnYMaxOffset`))) (+ (.z (.location _returnvalue_5)) (`KismetMathLibrary.RandomFloatInRange` (`self.HSpawnZMinOffset`) (`self.HSpawnZMaxOffset`)))) (`KismetMathLibrary.MakeRotator` _returnvalue_roll _returnvalue_pitch (+ (- _returnvalue_yaw (/ _spreadangle_2 2.0)) (* _index (/ _spreadangle_2 (`KismetMathLibrary.Conv_IntToDouble` (`self.NbSpreadShot`)))))) (`KismetMathLibrary.MakeVector` _returnvalue_4 _returnvalue_4 _returnvalue_4)) "Undefined" "OverrideRootScale" null self null))
                (`ParticleSystemComponent.SetTemplate` (`/Game/Enemy/AbilitySystem/BP_Ability.ParticleSystem` _returnvalue_9) "/Game/Enemy/AbilitySystem/Particles/PS_Fireball_2.PS_Fireball_2")
                (`KismetArrayLibrary.Array_Add` (`self.HomingArr`) _returnvalue_9))
              (`|PlayMontage` (`self.Mesh`) _shoming_animmontage_2 1.0 0.0 "None"
                (:`OnInterrupted`
                  (for _array_element _homingarr
                    (`/Engine/EditorBlueprintResources/StandardMacros.IsValid` _array_element
                      (:`Is Valid`
                        (`self.K2_DestroyActor` _array_element)))))
                (:`OnNotifyBegin`
                  (for _array_element_2 _homingarr
                    (`/Engine/EditorBlueprintResources/StandardMacros.IsValid` _array_element_2
                      (:`Is Valid`
                        (`/Game/Enemy/AbilitySystem/BP_Ability.CastAbility` _array_element_2)))))))
            (:`then_1`
              (set `self.didHoming` true)))))
      (else
        (`|ExecutionSequence`
          (:`then_0`
            ;;[1 1 1] Spread
            (`KismetArrayLibrary.Array_Clear` (`self.SpreadArr`))
            (for _index_2 (range (+ (`self.NbSpreadShot`) 1))
              (bind _returnvalue_10 (`|SpawnActorFromClass` "/Game/Enemy/AbilitySystem/Projectiles/BP_SpreadFireball.BP_SpreadFireball_C" (`KismetMathLibrary.MakeTransform` (.location _returnvalue_3) (`KismetMathLibrary.MakeRotator` (.roll (.rotation _returnvalue_3)) (.pitch (.rotation _returnvalue_3)) (+ (- (.yaw (.rotation _returnvalue_3)) (/ _spreadangle 2.0)) (* _index_2 (/ _spreadangle (`KismetMathLibrary.Conv_IntToDouble` (`self.NbSpreadShot`)))))) (.scale _returnvalue_3)) "Undefined" "OverrideRootScale" null self null))
              (`ParticleSystemComponent.SetTemplate` (`/Game/Enemy/AbilitySystem/BP_Ability.ParticleSystem` _returnvalue_10) "/Game/Enemy/AbilitySystem/Particles/PS_Fireball_2.PS_Fireball_2")
              (`KismetArrayLibrary.Array_Add` (`self.SpreadArr`) _returnvalue_10))
            (`|PlayMontage` (`self.Mesh`) _sspread_animmontage_2 1.0 0.0 "None"
              (:`OnInterrupted`
                (for _array_element_3 (`self.SpreadArr`)
                  (`/Engine/EditorBlueprintResources/StandardMacros.IsValid` _array_element_3
                    (:`Is Valid`
                      (`self.K2_DestroyActor` _array_element_3)))))
              (:`OnNotifyBegin`
                (`GameplayStatics.PlaySound2D` _sspread_sound 1.0 1.0 0.0 null null)
                (for _array_element_4 (`self.SpreadArr`)
                  (`/Engine/EditorBlueprintResources/StandardMacros.IsValid` _array_element_4
                    (:`Is Valid`
                      (`/Game/Enemy/AbilitySystem/BP_Ability.CastAbility` _array_element_4)))))))
          (:`then_1`
            (set `self.didSpread` true)))))
    (else
      (`|ExecutionSequence`
        (:`then_0`
          ;;[1 1 1] Fireball
          (`|PlayMontage` (`self.Mesh`) _sfireball_animmontage 0.5 0.0 "None"
            (:`OnCompleted`
              _)
            (:`OnNotifyBegin`
              _))
          (bind _returnvalue_11 (`GameplayStatics.SpawnSound2D` _sfireball_sound 1.0 1.0 0.0 null))
          (set `self.FSoundRef` _returnvalue_11)
          (bind _returnvalue_12 (`|SpawnActorFromClass` "/Game/Enemy/AbilitySystem/Projectiles/BP_Fireball.BP_Fireball_C" (`KismetMathLibrary.MakeTransform` (`KismetMathLibrary.MakeVector` (.x (.location _returnvalue)) (.y (.location _returnvalue)) (+ (.z (.location _returnvalue)) (`self.FireballZOffset`))) (.rotation _returnvalue) (.scale _returnvalue)) "Undefined" "OverrideRootScale" null self null))
          (`ParticleSystemComponent.SetTemplate` (`/Game/Enemy/AbilitySystem/BP_Ability.ParticleSystem` _returnvalue_12) "/Game/Enemy/AbilitySystem/Particles/PS_Fireball_2.PS_Fireball_2")
          (`/Game/Enemy/AbilitySystem/BP_Ability.CastAbility` _returnvalue_12)
          (bind _fsoundref (`self.FSoundRef`)
            (:`then`
              (`ActorComponent.K2_DestroyComponent` _fsoundref))
            (:`else`)))
        (:`then_1`
          (set `self.didFireball` true))))))

(event `self.ReceiveBeginPlay`
  ;[1 1 1] setup
  (`parent.ReceiveBeginPlay`)
  (set `self.delay` (`self.InitialDelay`))
  (set `self.Health` (`self.MaxHealth`))
  (`AudioComponent.Play` (`self.Beat`) 0.0)
  (`KismetSystemLibrary.Delay` (`self.DelayBetweenPist`))
  (`AudioComponent.Play` (`self.Music`) 0.0))

(event `self.ReceiveTick`
  (params (DeltaSeconds :type "Float (single-precision)"))
  (bind _delay (`self.delay`))
  ;[1 1 1] Sound
  (`parent.ReceiveTick` 0.0)
  (`|ExecutionSequence`
    (:`then_0`
      (set `self.TimePassed` (+ (`self.TimePassed`) (`GameplayStatics.GetWorldDeltaSeconds`)))
      (if (<= _delay 0.0)
        (if (>= (`self.TimePassed`) 44.0)
          (`/Engine/EditorBlueprintResources/StandardMacros.DoOnce` false
            (:`Completed`
              (set `self.WhiteToGreen` 0.0)
              (set `self.GreenDuration` 0.2)
              (set `self.Rate` 5.0)
              (set `self.Rate` 6.0))))
        (else
          (set `self.delay` (- _delay (`GameplayStatics.GetWorldDeltaSeconds`))))))
    (:`then_1`
      (if (not (`self.CanBeHit`))
        (`PrimitiveComponent.SetMaterial` (`self.Mesh`) 0 "/Game/AnimBoss/asset_3D/Material/01_Boss_V1_Black.01_Boss_V1_Black")))))

(event `self.Beat.OnAudioSingleEnvelopeValue`
  (params (PlayingSoundWave :type "SoundWave Object Reference") (EnvelopeValue :type "Float (single-precision)"))
  (bind _delay (`self.delay`))
  (bind _mesh (`self.Mesh`))
  ;[1 1 1] Sound
  (if (and (> EnvelopeValue 0.4) (<= _delay 0.0))
    (set `self.CanBeHit` true)
    (set `self.SoonHit` true)
    (set `self.delay` (`self.InitialDelay`))
    (`PrimitiveComponent.SetMaterial` _mesh 0 "/Game/Enemy/Boss_2/Material__16.Material__16")
    (bind _asfirst_person_character (cast `/Game/FirstPersonBP/Blueprints/FirstPersonCharacter` (`GameplayStatics.GetPlayerCharacter` 0)))
    (`TimelineComponent.SetPlayRate` (`self.Timeline_0`) (`self.Rate`))
    (bind (_direction _marker) (`Timeline|Timeline_0` :!via `PlayFromStart`)
      (:`Update`
        (bind _marker2 (`/Game/UI/Player_UI.marker2` (`/Game/FirstPersonBP/Blueprints/FirstPersonCharacter.PlayerUI_Ref` _asfirst_person_character)))
        (`Widget.SetRenderScale` _marker2 (* (1.0 1.0) _marker))
        (`KismetSystemLibrary.Delay` (`self.WhiteToGreen`))
        (set `self.SoonHit` false)
        (`PrimitiveComponent.SetMaterial` _mesh 0 "/Game/Enemy/Boss_2/Material__17.Material__17")
        (`Image.SetColorAndOpacity` _marker2 (struct :`G` 1.0 :`B` 0.025283 :`A` 1.0))
        (`KismetSystemLibrary.Delay` (`self.GreenDuration`))
        (set `self.CanBeHit` false)
        (`Widget.SetRenderScale` _marker2 (0.0 0.0))
        (`Image.SetColorAndOpacity` _marker2 (struct :`R` 1.0 :`G` 1.0 :`B` 1.0 :`A` 1.0))))
    (else
      (set `self.delay` (- _delay (`GameplayStatics.GetWorldDeltaSeconds`))))))

(fn `UserConstructionScript`
  (`parent.UserConstructionScript`))