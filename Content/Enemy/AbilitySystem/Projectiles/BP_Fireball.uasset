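; Enemy fireball projectile ability that explodes on impact and damages the first-person player.
; CastAbility runs the parent logic, then starts a 2D fire sound that is stopped when the actor is destroyed.
; Sphere overlap ignores other fireballs and BP_Character actors; any other actor triggers a scaled-up explosion emitter and destroys the projectile, applying Damage only to FirstPersonCharacter.
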(event `self.CastAbility`
  (`parent.CastAbility`)
  (bind _returnvalue (`GameplayStatics.SpawnSound2D` "/Game/StarterContent/Audio/Fire01_Cue.Fire01_Cue" 1.0 1.0 0.0 null))
  (add `self.OnDestroyed` (delegate `CustomEvent_0`)))

(event `CustomEvent_0` :!signature `self.OnDestroyed`
  (params (DestroyedActor :type "Actor Object Reference"))
  (`/Engine/EditorBlueprintResources/StandardMacros.IsValid` (stale `self.CastAbility` _returnvalue)
    (:`Is Valid`
      (`ActorComponent.K2_DestroyComponent` (stale `self.CastAbility` _returnvalue)))))

(event `self.Sphere.OnComponentBeginOverlap`
  (params (OverlappedComponent :type "PrimitiveComponent Object Reference") (OtherActor :type "Actor Object Reference") (OtherComp :type "PrimitiveComponent Object Reference") (OtherBodyIndex :type Integer) (bFromSweep :type Boolean) (SweepResult :type "HitResult Structure (by ref)"))
  (cast `/Game/Enemy/AbilitySystem/Projectiles/BP_Fireball` OtherActor
    (:`CastFailed`
      (cast `/Game/Enemy/BP_Character` OtherActor
        (:`CastFailed`
          (`GameplayStatics.SpawnEmitterAtLocation` "/Game/StarterContent/Particles/P_Explosion.P_Explosion" (`SceneComponent.K2_GetComponentLocation` (`self.DefaultSceneRoot`)) (struct) (5.0 5.0 5.0))
          (bind _asfirst_person_character (cast `/Game/FirstPersonBP/Blueprints/FirstPersonCharacter` OtherActor)
            (:`then`
              (`GameplayStatics.ApplyDamage` _asfirst_person_character (`self.Damage`)))
            (:`CastFailed`
              _))
          (`self.K2_DestroyActor`))))))

(fn `UserConstructionScript`
  (`parent.UserConstructionScript`))