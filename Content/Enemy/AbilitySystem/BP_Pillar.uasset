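; Enemy pillar ability that erupts after a telegraphed charge and damages the player.
; CastAbility plays charge, upheaval and shatter particle effects in delayed stages, then sets HasCast.
; Tick then sets the hit box's Z scale toward MaxZHeight through FInterpTo and destroys the actor after a delay.
; Box overlap applies damage to the FirstPersonCharacter, gated by DoOnce so it lands only once.
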(event `self.CastAbility`
  (`parent.CastAbility`)
  (`ActorComponent.Activate` (`self.PS_UpvealCharge`) false)
  (`KismetSystemLibrary.Delay` (`self.DelayBeforeUpveal`))
  (`ActorComponent.Activate` (`self.ParticleSystem`) false)
  (`KismetSystemLibrary.Delay` (`self.DelayBeforeShatter`))
  (`ActorComponent.Activate` (`self.PS_AuraShatter`) false)
  (`ActorComponent.Activate` (`self.PS_End`) false)
  (set `self.hasCast` true))

(event `self.ReceiveTick`
  (params (DeltaSeconds :type "Float (single-precision)"))
  (bind _box (`self.Box`))
  (bind (_returnvalue_x _returnvalue_y _returnvalue_z) (`KismetMathLibrary.BreakVector` (`SceneComponent.K2_GetComponentScale` _box)))
  (if (`self.hasCast`)
    (`SceneComponent.SetWorldScale3D` _box (`KismetMathLibrary.MakeVector` _returnvalue_x _returnvalue_y (`KismetMathLibrary.FInterpTo` _returnvalue_z (`self.MaxZHeight`) DeltaSeconds)))
    (`KismetSystemLibrary.Delay` (`self.DelayBeforeDestroy`))
    (`self.K2_DestroyActor`)))

(event `self.Box.OnComponentBeginOverlap`
  (params (OverlappedComponent :type "PrimitiveComponent Object Reference") (OtherActor :type "Actor Object Reference") (OtherComp :type "PrimitiveComponent Object Reference") (OtherBodyIndex :type Integer) (bFromSweep :type Boolean) (SweepResult :type "HitResult Structure (by ref)"))
  (bind _asfirst_person_character (cast `/Game/FirstPersonBP/Blueprints/FirstPersonCharacter` OtherActor))
  (`/Engine/EditorBlueprintResources/StandardMacros.DoOnce` false
    (:`Completed`
      (`GameplayStatics.ApplyDamage` _asfirst_person_character (`self.Damage`)))))

(fn `UserConstructionScript`
  (`parent.UserConstructionScript`))