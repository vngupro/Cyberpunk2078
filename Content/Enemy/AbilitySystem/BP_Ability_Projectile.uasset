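; Projectile ability actor that rides on the caster's left-hand socket until cast, then launches as a spinning projectile.
; Construction sets movement speed from the ability details, attaches to the caster's mesh and binds to the character's death event.
; CastAbility runs the parent logic, detaches in world space and activates projectile movement.
; Once launched, Tick adds a fixed roll step each frame, so spin rate depends on frame rate.
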(event `self.CastAbility`
  (`parent.CastAbility`)
  (`self.K2_DetachFromActor` "KeepWorld" "KeepWorld" "KeepWorld")
  (`ActorComponent.Activate` (`self.ProjectileMovement`) true)
  (set `self.hasLaunch` true))

(event `self.ReceiveTick`
  (params (DeltaSeconds :type "Float (single-precision)"))
  (bind (_returnvalue_roll _returnvalue_pitch _returnvalue_yaw) (`KismetMathLibrary.BreakRotator` (`self.K2_GetActorRotation`)))
  (if (`self.hasLaunch`)
    (`self.K2_SetActorRotation` (`KismetMathLibrary.MakeRotator` (+ _returnvalue_roll (`self.RotationSpeed`)) _returnvalue_pitch _returnvalue_yaw))))

(fn `UserConstructionScript`
  (bind _projectilemovement (`self.ProjectileMovement`))
  (bind (_abilitydetails_name _abilitydetails_description _abilitydetails_cost _abilitydetails_cooldown _abilitydetails_casttime _abilitydetails_speed) (break `/Game/Enemy/AbilitySystem/SAbilityDetails` (`self.AbilityDetails`)))
  (bind _caster (`self.Caster`))
  (`parent.UserConstructionScript`)
  (set `ProjectileMovementComponent.MaxSpeed` _abilitydetails_speed _projectilemovement)
  (set `ProjectileMovementComponent.InitialSpeed` _abilitydetails_speed _projectilemovement)
  (`self.K2_AttachToComponent` (`Character.Mesh` _caster) "ProjectileLeftHand" "SnapToTarget" "KeepWorld" "SnapToTarget")
  (bind _asbp_character (cast `/Game/Enemy/BP_Character` _caster))
  (set `self.CharacterRef` _asbp_character)
  (add `/Game/Enemy/BP_Character.IAmDead` _asbp_character (`|CreateDelegate` :!event `InteruptCasting`)))