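; Area-of-effect enemy ability actor that, once cast, activates its particle system and enlarges until it destroys itself.
; Each tick after launch sets actor X/Y scale via FInterpTo toward MaxSize, with X's zero interp speed snapping straight to it.
; The Box's world X/Y scale follows actor X scale plus an offset that grows per tick, with fixed ZHeight.
; Lifetime is a tick counter compared against DelayBeforeDestroy divided by DeltaSeconds.
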(event `self.ReceiveBeginPlay`
  (`parent.ReceiveBeginPlay`))

(event `self.CastAbility`
  (`parent.CastAbility`)
  (`ActorComponent.Activate` (`self.ParticleSystem`) true)
  (set `self.hasLaunch` true))

(event `self.ReceiveTick`
  (params (DeltaSeconds :type "Float (single-precision)"))
  (bind (_returnvalue_x _returnvalue_y _returnvalue_z) (`KismetMathLibrary.BreakVector` (`self.GetActorScale3D`)))
  (bind _returnvalue_x_2 (`KismetMathLibrary.BreakVector` (`self.GetActorScale3D`)))
  (bind _deathcount (`self.DeathCount`))
  (bind _resizecount (`self.ResizeCount`))
  (bind _returnvalue (+ _returnvalue_x_2 _resizecount))
  (if (`self.hasLaunch`)
    (`self.SetActorScale3D` (`KismetMathLibrary.MakeVector` (`KismetMathLibrary.FInterpTo` _returnvalue_x (`self.MaxSize`) DeltaSeconds 0.0) (`KismetMathLibrary.FInterpTo` _returnvalue_y (`self.MaxSize`) DeltaSeconds) _returnvalue_z))
    (`SceneComponent.SetWorldScale3D` (`self.Box`) (`KismetMathLibrary.MakeVector` _returnvalue _returnvalue (`self.ZHeight`)))
    (set `self.ResizeCount` (+ _resizecount (`self.ResizeCountIncrementalFactor`)))
    (`/Engine/EditorBlueprintResources/StandardMacros.IncrementFloat` _deathcount
      (:`  `
        (if (>= _deathcount (/ (`self.DelayBeforeDestroy`) DeltaSeconds))
          (`self.K2_DestroyActor`))))))

(fn `UserConstructionScript`
  (`parent.UserConstructionScript`))